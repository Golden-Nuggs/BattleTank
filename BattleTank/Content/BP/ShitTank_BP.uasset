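; Player-controllable tank Blueprint with independently throttled left and right tracks, an orbiting aim camera rig and cannon firing.
; BeginPlay passes the barrel and turret components to inherited or external setter functions.
; Input axes rotate the azimuth gimbal in yaw and the spring arm in pitch, and drive each track's throttle separately.
; The fire action calls FireCannons, whose logic lives outside these graphs.
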(event EventBeginPlay
  (Class|Tank|SetBarrelReference (Variables|Default|GetTankBarrel))
  (Class|Tank|SetTurretReference (Variables|Default|GetTankTurret)))

(event Input|ActionEvents|InputActionFireProjectile
  (params (Key :type Key%20Structure :default "None"))
  ;[1 1 1] Action Key Bindings
  (:Pressed
    (Class|Tank|FireCannons)))

(event Input|AxisEvents|InputAxisAimAzimuth
  (params (AxisValue :type Float%20%28single-precision%29))
  ;[1 1 1] Aim Axis Bindings
  (Transformation|AddLocalRotation (Variables|Default|GetAzimuth%20Gimbal) (Math|Rotator|MakeRotator 0.0 0.0 AxisValue) false false))

(event Input|AxisEvents|InputAxisAimElevation
  (params (AxisValue :type Float%20%28single-precision%29))
  ;[1 1 1] Aim Axis Bindings
  (Transformation|AddLocalRotation (Variables|Default|GetSpring%20Arm) (Math|Rotator|MakeRotator 0.0 AxisValue 0.0) false false))

(event Input|AxisEvents|InputAxisLeftTrackThrottle
  (params (AxisValue :type Float%20%28single-precision%29))
  ;[1 1 1] Throttle Axis Bindings
  (Class|TankTrack|SetThrottle (Variables|Default|GetTankTrack_L) AxisValue))

(event Input|AxisEvents|InputAxisRightTrackThrottle
  (params (AxisValue :type Float%20%28single-precision%29))
  ;[1 1 1] Throttle Axis Bindings
  (Class|TankTrack|SetThrottle (Variables|Default|GetTankTrack_R) AxisValue))

(fn ConstructionScript)